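; Squad member character Blueprint that carries a weapon through a DefaultWeapon child actor and currently only visualises its hand alignment.
; Every Tick it draws debug spheres at the weapon's GripPoint socket and at the character mesh's hand_r_WeaponSocket.
; The construction script is empty, with disconnected, never-run nodes left over for offsetting the weapon by its grip socket position.
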(event `self.ReceiveTick`
  (params (DeltaSeconds :type "Float (single-precision)"))
  (`|ExecutionSequence`
    (:`then_0`
      (bind _childactor (`ChildActorComponent.ChildActor` (`self.DefaultWeapon`))
        (:`then`
          (bind _asweapon_base (cast `WeaponBase` _childactor))
          (`KismetSystemLibrary.DrawDebugSphere` (`SceneComponent.GetSocketLocation` (`WeaponBase.WeaponMesh` _asweapon_base) "GripPoint") 5.0 12 (struct :`R` 1.0 :`G` 1.0 :`B` 1.0 :`A` 1.0) 0.0 1.0))
        (:`else`)))
    (:`then_1`
      (`KismetSystemLibrary.DrawDebugSphere` (`SceneComponent.GetSocketLocation` (`self.Mesh`) "hand_r_WeaponSocket") 5.0 12 (struct :`R` 1.0 :`B` 0.86183 :`A` 1.0) 0.0 1.0))))

(fn `UserConstructionScript`)