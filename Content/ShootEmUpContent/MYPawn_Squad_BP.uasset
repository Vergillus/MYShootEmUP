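; Squad pawn for a shoot 'em up that holds squad members as child actors and sets up their health HUD.
; On BeginPlay it creates MainHUD_WBP and subscribes each health bar, by index, to the matching member's HealthComponent.
; Pressing X damages every member, apparently as a test input.
; Logic to turn LeaderText along the camera's horizontal forward vector is left unconnected, and Tick is empty.
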(event `self.ReceiveBeginPlay`
  (bind _squadmembers (`self.SquadMembers`))
  (bind _returnvalue (`|CreateWidget` "/Game/ShootEmUpContent/Widgets/MainHUD_WBP.MainHUD_WBP_C"))
  (`UserWidget.AddToViewport` _returnvalue 0)
  (for _index (range (`KismetArrayLibrary.Array_Length` _squadmembers))
    (`HealthBarUserWidget.SubscribeOnHealthChange` (`|GetArrayItem` (`/Game/ShootEmUpContent/Widgets/MainHUD_WBP.HealthBars` _returnvalue) _index) (`self.GetComponentByClass` (`ChildActorComponent.ChildActor` (`|GetArrayItem` _squadmembers _index)) "/Script/MYShootEmUp.HealthComponent"))))

(event `self.ReceiveTick`
  (params (DeltaSeconds :type "Float (single-precision)")))

(event `Key|X`
  (params (Key :type "Key Structure"))
  (:`Pressed`
    (for _array_element (`self.SquadMembers`)
      (`HealthComponent.DamageHealth` (`self.GetComponentByClass` (`ChildActorComponent.ChildActor` _array_element) "/Script/MYShootEmUp.HealthComponent") self 1.0))))

(fn `UserConstructionScript`)