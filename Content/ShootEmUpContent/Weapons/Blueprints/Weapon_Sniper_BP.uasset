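; Sniper weapon Blueprint that draws a laser-sight style aim line while its mesh is visible.
; Each Tick it draws a debug line from the muzzle socket along its forward vector out to FireRange, with no trace, so the line passes through obstacles.
; The owner, cast to MYCharacterBase, sets the color: blue for the leader, red otherwise.
; The sight relies on DrawDebugLine rather than a beam or mesh component.
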(event `self.ReceiveTick`
  (params (DeltaSeconds :type "Float (single-precision)"))
  (bind (_returnvalue_location _returnvalue_rotation) (`KismetMathLibrary.BreakTransform` (`SceneComponent.GetSocketTransform` (`self.WeaponMesh`) (`self.MuzzleSocketName`) "RTS_World")))
  (bind _returnvalue (+ _returnvalue_location (* (`KismetMathLibrary.GetForwardVector` _returnvalue_rotation) (`self.FireRange`))))
  (if (`SceneComponent.IsVisible` (`self.WeaponMesh`))
    (bind _asmycharacter_base (cast `MYCharacterBase` (`self.GetOwner`)))
    (if (`MYCharacterBase.bIsLeader` _asmycharacter_base)
      (`KismetSystemLibrary.DrawDebugLine` _returnvalue_location _returnvalue (struct :`G` 0.047142 :`B` 1.0 :`A` 1.0) 0.0 5.0)
      (else
        (`KismetSystemLibrary.DrawDebugLine` _returnvalue_location _returnvalue (struct :`R` 1.0 :`A` 1.0) 0.0 5.0)))))

(fn `UserConstructionScript`)