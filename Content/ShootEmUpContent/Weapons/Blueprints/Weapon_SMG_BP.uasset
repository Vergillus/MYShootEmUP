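; Weapon_SMG_BP is the submachine gun weapon Blueprint in the ShootEmUp content.
; Each Tick, while the weapon mesh is visible, it draws a red debug line from the muzzle socket along its forward vector for the length of FireRange, like a laser sight.
; The graph contains no firing logic, and BeginPlay, ActorBeginOverlap and the construction script are empty.
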(event `self.ReceiveTick`
  (params (DeltaSeconds :type "Float (single-precision)"))
  (bind (_returnvalue_location _returnvalue_rotation) (`KismetMathLibrary.BreakTransform` (`SceneComponent.GetSocketTransform` (`self.WeaponMesh`) (`self.MuzzleSocketName`) "RTS_World")))
  (if (`SceneComponent.IsVisible` (`self.WeaponMesh`))
    (`KismetSystemLibrary.DrawDebugLine` _returnvalue_location (+ _returnvalue_location (* (`KismetMathLibrary.GetForwardVector` _returnvalue_rotation) (`self.FireRange`))) (struct :`R` 1.0 :`A` 1.0) 0.0 2.0)))

(fn `UserConstructionScript`)